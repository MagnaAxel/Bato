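; OBJ_Catch is a timed direction-sequence challenge object, apparently for a catch mechanic.
; Play starts a delayed timer targeting an End function, and Catch advances an index only when the given direction matches the current Sequence entry, ignoring wrong inputs.
; GetDirection exposes the expected direction as a string, or "None" once complete.
; Finish fires OnFinished with whether the whole sequence was matched.
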(fn `Catch`
  (params (Direction :type "/Game/Database/EN_Direction Enum (by ref)"))
  (if (< (`self.Index`) (`KismetArrayLibrary.Array_Length` (`self.Sequence`)))
    (if (`|EnumEquality` (`|GetArrayItem` (`self.Sequence`) (`self.Index`)) Direction)
      (`/Engine/EditorBlueprintResources/StandardMacros.IncrementInt` (`self.Index`)))))

(fn `Finish`
  (`self.OnFinished` (== (`self.Index`) (`KismetArrayLibrary.Array_Length` (`self.Sequence`)))))

(fn `GetDirection`
  (returns (ReturnValue :type String))
  (return (select `bool` (< (`self.Index`) (`KismetArrayLibrary.Array_Length` (`self.Sequence`))) :`true` (`|GetEnumeratorNameAsString` (`|GetArrayItem` (`self.Sequence`) (`self.Index`))))))

(fn `Play`
  (bind _returnvalue (`KismetSystemLibrary.K2_SetTimer` null "End" (`self.Delay`)))
  (set `self.Timer` _returnvalue))
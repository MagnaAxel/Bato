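; Actor component that makes its owner float on waves.
; Every tick it fetches wave data from the GameState through an interface and evaluates wave height and normal at the owner's XY position.
; It interpolates the owner toward that height minus Deepness at Buoyancy speed, and tilts it to the wave normal at Stability speed, keeping its forward heading and sweeping for collisions.
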(event `self.ReceiveTick`
  (params (DeltaSeconds :type "Float (single-precision)"))
  (bind _returnvalue (`self.GetOwner`))
  (bind _returnvalue_2 (`Actor.K2_GetActorLocation` _returnvalue))
  (bind _returnvalue_3 (`KismetMathLibrary.Conv_VectorToVector2D` _returnvalue_2))
  (bind _wave (message `/Game/Blueprints/System/IN_GSB_Bato.IGetWave` (`GameplayStatics.GetGameState`) _returnvalue_3))
  (bind (_height _normal) (`/Game/Blueprints/FL_Wave.GetWave` _returnvalue_3 _wave))
  (`Actor.K2_SetActorLocationAndRotation` _returnvalue (`KismetMathLibrary.VInterpTo` _returnvalue_2 (`KismetMathLibrary.Conv_Vector2DToVector` _returnvalue_3 (- _height (`self.Deepness`))) (`GameplayStatics.GetWorldDeltaSeconds`) (`self.Buoyancy`)) (`KismetMathLibrary.RInterpTo` (`Actor.K2_GetActorRotation` _returnvalue) (`KismetMathLibrary.MakeRotFromZX` _normal (`Actor.GetActorForwardVector` _returnvalue)) (`GameplayStatics.GetWorldDeltaSeconds`) (`self.Stability`)) true false))
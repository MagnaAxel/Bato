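; BP_FishingRod is a fishing rod that runs a timed directional-pull minigame and gives caught fish to its owner.
; Cast toggles fishing, animating hook and line via a timeline and starting a bite timer scaled by fish zone.
; Bites pick a fish by biome, weather and period, opening a rarity-timed window to match its pull sequence.
; Pulls trigger force feedback, callbacks report progress, and each window's end restarts the wait.
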(event `self.ReceiveBeginPlay`
  (message `/Game/Blueprints/IN_ObjectWidget.SetObjectWidget` (`WidgetComponent.GetWidget` (`self.WI_FishingRod`)) self))

(fn `Abort`
  (`KismetSystemLibrary.K2_ClearAndInvalidateTimerHandle` (`self.FishingTimer`))
  (`KismetSystemLibrary.K2_ClearAndInvalidateTimerHandle` (`self.PullTimer`))
  (set `self.Fishing` false)
  (`self.OnAbortedFishing`))

(fn `Cast`
  (returns (Success :type Boolean))
  (if (not (`self.Fishing`))
    (`TimelineComponent.Play` (`self.TimelineFishing`))
    (`self.Fish`)
    (else
      (`TimelineComponent.Reverse` (`self.TimelineFishing`))
      (`self.Abort`)))
  (return true))

(fn `End`
  (bind _returnvalue (== (`self.PullIndex`) (`KismetArrayLibrary.Array_Length` (`self.Pulls`))))
  (`|ExecutionSequence`
    (:`then_0`
      (if _returnvalue
        (message `/Game/Blueprints/Gameplay/Cargo/IN_Cargo.AddFish` (`self.GetOwner`) (`self.PullFish`))))
    (:`then_1`
      (`self.OnEndedFishing` _returnvalue))
    (:`then_2`
      (`self.Fish`))))

(fn `Fish`
  (bind _returnvalue (`KismetSystemLibrary.K2_SetTimer` null "Start" (`KismetMathLibrary.Lerp` (`self.MaxFishingDelay`) (`self.MinFishingDelay`) (`/Game/Database/FishZone/FL_FishZone.GetFishZone` (`KismetMathLibrary.Conv_VectorToVector2D` (`self.K2_GetActorLocation`))))))
  (set `self.FishingTimer` _returnvalue)
  (set `self.Fishing` true))

(fn `GetFishingTimer`
  (returns (FishingTimer :type "TimerHandle Structure"))
  (return (`self.FishingTimer`)))

(fn `GetPull`
  (returns (Pull :type "/Game/Database/EN_Pull Enum"))
  (bind _pulls (`self.Pulls`))
  (bind _pullindex (`self.PullIndex`))
  (return (select `bool` (`KismetArrayLibrary.Array_IsValidIndex` _pulls _pullindex) :`false` "NewEnumerator5" :`true` (`|GetArrayItem` _pulls _pullindex))))

(fn `GetPullFish`
  (returns (PullFish :type "/Game/Database/Fish/EN_Fish Enum"))
  (return (`self.PullFish`)))

(fn `GetPullPercent`
  (returns (PullPercent :type "Float (double-precision)"))
  (return (/ (`self.PullIndex`) (`KismetArrayLibrary.Array_Length` (`self.Pulls`)))))

(fn `GetPullTimer`
  (returns (PullTimer :type "TimerHandle Structure"))
  (return (`self.PullTimer`)))

(fn `IsFishing`
  (returns (Fishing :type Boolean))
  (return (`self.Fishing`)))

(fn `Pull`
  (params (Direction :type "/Game/Database/EN_Pull Enum" :default "NewEnumerator5"))
  (returns (Success :type Boolean))
  (locals (LocalSuccess :type Boolean))
  (bind _pulltimer (`self.PullTimer`))
  (bind _returnvalue (`KismetSystemLibrary.K2_GetTimerElapsedTimeHandle` _pulltimer))
  (if (and (`KismetSystemLibrary.K2_IsTimerActiveHandle` (`self.PullTimer`)) (< (`self.PullIndex`) (`KismetArrayLibrary.Array_Length` (`self.Pulls`))))
    (bind _output_get (set `local.LocalSuccess` (`|EnumEquality` (`|GetArrayItem` (`self.Pulls`) (`self.PullIndex`)) Direction)))
    (`|ExecutionSequence`
      (:`then_0`
        (if _output_get
          (`/Engine/EditorBlueprintResources/StandardMacros.IncrementInt` (`self.PullIndex`))))
      (:`then_1`
        (`ForceFeedbackComponent.SetIntensityMultiplier` (`self.ForceFeedback`) (/ _returnvalue (+ _returnvalue (`KismetSystemLibrary.K2_GetTimerRemainingTimeHandle` _pulltimer))))
        (`ForceFeedbackComponent.Play` (`self.ForceFeedback`) 0.0))
      (:`then_2`
        (`self.OnPulledFishing` _output_get))
      (:`then_3`
        (return _output_get)))
    (else
      (return false))))

(fn `Start`
  (bind _fish (`/Game/Database/Fish/FL_Fish.GetFish` (`/Game/Database/Fish/FL_Fish.GetRandomFish` (`/Game/Database/Biome/FL_Biome.GetBiome` (`KismetMathLibrary.Conv_VectorToVector2D` (`self.K2_GetActorLocation`))) (`/Game/Database/Weather/FL_Weather.GetActiveWeather`) (`/Game/Database/Time/FL_Time.GetPeriod`))))
  (bind ((`Name_4_6C28D4E14EC300F6584FDFAAD19B9B59` _name) (`Rarity_6_44CFD01B4BB894FA46BFC3A734ED8C18` _rarity) (`Pulls_23_842178DD430B09C21B924EBB62C0A6BB` _pulls)) (break `/Game/Database/Fish/ST_Fish` _fish))
  (set `self.PullFish` _name)
  (set `self.Pulls` _pulls)
  (set `self.PullIndex` 0)
  (bind _returnvalue (`KismetSystemLibrary.K2_SetTimer` null "End" (`.GrabDelay_12_29807F4C437A7F2EBBBFC6A4A7663009` (break `/Game/Database/Rarity/ST_Rarity` (`/Game/Database/Rarity/FL_Rarity.GetRarity` _rarity)))))
  (set `self.PullTimer` _returnvalue)
  (`self.OnStartedFishing`))

(fn `UserConstructionScript`)
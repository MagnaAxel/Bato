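; BP_Cannon is a cannon actor that fires BP_Cannonball projectiles with a reload delay between shots.
; Shoot spawns a ball at the CannonballTransform component, with velocity set to the actor's forward vector scaled by Impulse.
; The reload timer handle doubles as the cooldown flag: Shoot fires only while it is invalid, and Reload clears it.
; SetStrength is a stub that returns false.
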(fn `Reload`
  (`KismetSystemLibrary.K2_ClearAndInvalidateTimerHandle` (`self.ReloadTimer`)))

(fn `SetStrength`
  (params (Strength :type Integer))
  (returns (Success :type Boolean))
  (return false))

(fn `Shoot`
  (returns (Success :type Boolean))
  (if (not (`KismetSystemLibrary.K2_IsValidTimerHandle` (`self.ReloadTimer`)))
    (`|SpawnActorFromClass` "/Game/Blueprints/Gameplay/Cannon/BP_Cannonball.BP_Cannonball_C" (`SceneComponent.K2_GetComponentToWorld` (`self.CannonballTransform`)) "AlwaysSpawn" "MultiplyWithRoot" null (* (`self.GetActorForwardVector`) (`self.Impulse`)) null)
    (bind _returnvalue (`KismetSystemLibrary.K2_SetTimer` null "Reload" (`self.ReloadDelay`)))
    (set `self.ReloadTimer` _returnvalue)
    (return true)))

(fn `UserConstructionScript`)
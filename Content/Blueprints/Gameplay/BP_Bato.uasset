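; BP_Bato is a movable boat pawn that floats on waves and drifts with their slope.
; Each tick, Float samples wave height and normal from the GameState at its position.
; It interpolates actor height minus Deepness, tilts the static mesh toward the normal, and turns that tilt into drift input.
; Move adds forward input and steers by interpolating actor rotation, scaled by Maneuverability.
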(event `self.ReceiveTick`
  (params (DeltaSeconds :type "Float (single-precision)"))
  (`self.Float`))

(fn `Float`
  (bind _adrift (`self.Adrift`))
  (bind _returnvalue (`KismetMathLibrary.Conv_VectorToVector2D` (`self.K2_GetActorLocation`)))
  (`|ExecutionSequence`
    (:`then_0`
      (bind (_height _normal) (message `/Game/Blueprints/System/IN_Wave.GetWave` (`GameplayStatics.GetGameState`) _returnvalue))
      (`self.K2_SetActorLocation` (`KismetMathLibrary.VInterpTo` (`self.K2_GetActorLocation`) (`KismetMathLibrary.Conv_Vector2DToVector` _returnvalue (- _height (`self.Deepness`))) (`GameplayStatics.GetWorldDeltaSeconds`) (`self.Floatation`)) true))
    (:`then_1`
      (`SceneComponent.K2_SetWorldRotation` (`self.StaticMesh`) (`KismetMathLibrary.RInterpTo` (`SceneComponent.K2_GetComponentRotation` (`self.StaticMesh`)) (`KismetMathLibrary.MakeRotFromZX` _normal (`self.GetActorForwardVector`)) (`GameplayStatics.GetWorldDeltaSeconds`) (`self.Stability`)) false false))
    (:`then_2`
      (`self.AddMovementInput` (`KismetMathLibrary.MakeVector` (* (.pitch (`SceneComponent.K2_GetComponentRotation` (`self.StaticMesh`))) _adrift -1.0) (* (.roll (`SceneComponent.K2_GetComponentRotation` (`self.StaticMesh`))) _adrift))))))

(fn `Move`
  (params (Vector2D :type "Vector2D Structure"))
  (returns (Success :type Boolean))
  (bind (_x _y) (`KismetMathLibrary.BreakVector2D` Vector2D))
  (bind _returnvalue (`self.K2_GetActorRotation`))
  (`self.AddMovementInput` (* (`self.GetActorForwardVector`) _x))
  (`self.K2_SetActorRotation` (`KismetMathLibrary.RInterpTo` _returnvalue (`KismetMathLibrary.ComposeRotators` _returnvalue (* (struct :`Yaw` 90.0) _y)) (`self.Maneuverability`) (`GameplayStatics.GetWorldDeltaSeconds`)))
  (return true))

(fn `UserConstructionScript`)
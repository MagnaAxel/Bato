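; Equipped boat pawn that carries cargo, a fishing rod and a cannon as child actors and tracks its own damage.
; Quantity, fishing and shooting calls are forwarded as messages to the matching child actor.
; Damage changes route through SetDamage into ApplyDamage, which at a fixed threshold unpossesses the controller, restarts the player through the GameMode and destroys the boat.
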(fn `AddDamage`
  (params (Damage :type Integer))
  (returns (Success :type Boolean))
  (bind _success (`self.SetDamage` (+ (`self.Damage`) Damage)))
  (return _success))

(fn `AddQuantity`
  (params (Quantity :type Integer))
  (returns (Success :type Boolean))
  (bind _success (message `/Game/Blueprints/Gameplay/IN_Cargo.AddQuantity` (`ChildActorComponent.ChildActor` (`self.Cargo`)) Quantity))
  (return _success))

(fn `ApplyDamage`
  (if (>= (`self.Damage`) 3)
    (`|ExecutionSequence`
      (:`then_0`
        (bind _returnvalue (`self.GetController`))
        (`/Engine/EditorBlueprintResources/StandardMacros.IsValid` _returnvalue
          (:`Is Valid`
            (`Controller.UnPossess` _returnvalue)
            (`GameModeBase.RestartPlayer` (`GameplayStatics.GetGameMode`) _returnvalue))))
      (:`then_1`
        (`self.K2_DestroyActor`)))))

(fn `Fish`
  (returns (Success :type Boolean))
  (bind _success (message `/Game/Blueprints/Gameplay/IN_FishingRod.Fish` (`ChildActorComponent.ChildActor` (`self.FishingRod`))))
  (return _success))

(fn `GetDamage`
  (returns (Success :type Boolean) (Damage :type Integer))
  (return true (`self.Damage`)))

(fn `GetQuantity`
  (returns (Success :type Boolean) (Quantity :type Integer))
  (bind (_success _quantity) (message `/Game/Blueprints/Gameplay/IN_Cargo.GetQuantity` (`ChildActorComponent.ChildActor` (`self.Cargo`))))
  (return _success _quantity))

(fn `ResetDamage`
  (returns (Success :type Boolean))
  (bind _success (`self.SetDamage` 0))
  (return _success))

(fn `ResetQuantity`
  (returns (Success :type Boolean))
  (bind _success (message `/Game/Blueprints/Gameplay/IN_Cargo.ResetQuantity` (`ChildActorComponent.ChildActor` (`self.Cargo`))))
  (return _success))

(fn `SetDamage`
  (params (Damage :type Integer))
  (returns (Success :type Boolean))
  (set `self.Damage` Damage)
  (`self.ApplyDamage`)
  (return true))

(fn `SetQuantity`
  (params (Quantity :type Integer))
  (returns (Success :type Boolean))
  (bind _success (message `/Game/Blueprints/Gameplay/IN_Cargo.SetQuantity` (`ChildActorComponent.ChildActor` (`self.Cargo`)) Quantity))
  (return _success))

(fn `Shoot`
  (returns (Success :type Boolean))
  (bind _success (message `/Game/Blueprints/Gameplay/IN_Cannon.Shoot` (`ChildActorComponent.ChildActor` (`self.Cannon`))))
  (return _success))

(fn `UserConstructionScript`
  (`parent.UserConstructionScript`))
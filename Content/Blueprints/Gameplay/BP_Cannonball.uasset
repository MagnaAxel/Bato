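; BP_Cannonball is a projectile that falls under gravity and deals damage to what it hits.
; Each Tick, a Gravity helper updates its Velocity and returns an offset, which moves the actor by a swept SetActorLocation rather than a movement component.
; A Hit sends a damage message of 1 to the other actor and destroys the cannonball, which also destroys itself at or below world Z zero.
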(event `self.ReceiveTick`
  (params (DeltaSeconds :type "Float (single-precision)"))
  (bind (_returnvalue_x _returnvalue_y _returnvalue_z) (`KismetMathLibrary.BreakVector` (`self.K2_GetActorLocation`)))
  (bind (_location _newvelocity) (`/Game/Blueprints/FL_Gravity.Gravity` (`self.Velocity`)))
  (set `self.Velocity` _newvelocity)
  (`self.K2_SetActorLocation` (+ (`self.K2_GetActorLocation`) _location) true)
  (if (<= _returnvalue_z 0.0)
    (`self.K2_DestroyActor`)))

(event `self.ReceiveHit`
  (params (MyComp :type "PrimitiveComponent Object Reference") (Other :type "Actor Object Reference") (OtherComp :type "PrimitiveComponent Object Reference") (bSelfMoved :type Boolean) (HitLocation :type "Vector Structure") (HitNormal :type "Vector Structure") (NormalImpulse :type "Vector Structure") (Hit :type "HitResult Structure (by ref)"))
  (`|ExecutionSequence`
    (:`then_0`
      (message `/Game/Blueprints/Gameplay/IN_Damage.AddDamage` Other 1))
    (:`then_1`
      (`self.K2_DestroyActor`))))

(fn `UserConstructionScript`)
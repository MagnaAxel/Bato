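; BP_Cargo is a fish cargo hold that stores fish up to a maximum and displays how full it is.
; ApplyFishes shows one of four cargo components per stored fish, running on construction and after each change.
; AddFish appends while space remains, calls CallOnAddedFish, and returns whether space is left afterwards.
; RemoveFish finds and removes a given fish, then refreshes the visuals.
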(fn `AddFish`
  (params (Fish :type "/Game/Database/Fish/EN_Fish Enum" :default "NewEnumerator0"))
  (returns (Success :type Boolean))
  (bind _returnvalue (< (`KismetArrayLibrary.Array_Length` (`self.Fishes`)) (`self.MaxFishes`)))
  (if _returnvalue
    (`KismetArrayLibrary.Array_Add` (`self.Fishes`) Fish)
    (`self.ApplyFishes`)
    (`self.OnAddedFish`))
  (return _returnvalue))

(fn `ApplyFishes`
  (bind _returnvalue (`KismetArrayLibrary.Array_Length` (`self.Fishes`)))
  (`|ExecutionSequence`
    (:`then_0`
      (`SceneComponent.SetHiddenInGame` (`self.Cargo1`) (<= _returnvalue 0) false))
    (:`then_1`
      (`SceneComponent.SetHiddenInGame` (`self.Cargo2`) (<= _returnvalue 1) false))
    (:`then_2`
      (`SceneComponent.SetHiddenInGame` (`self.Cargo3`) (<= _returnvalue 2) false))
    (:`then_3`
      (`SceneComponent.SetHiddenInGame` (`self.Cargo4`) (<= _returnvalue 3) false))))

(fn `RemoveFish`
  (params (Fish :type "/Game/Database/Fish/EN_Fish Enum" :default "NewEnumerator0"))
  (returns (Success :type Boolean))
  (bind _returnvalue (`KismetArrayLibrary.Array_Find` (`self.Fishes`) Fish))
  (bind _returnvalue_2 (>= _returnvalue 0))
  (if _returnvalue_2
    (`KismetArrayLibrary.Array_Remove` (`self.Fishes`) _returnvalue)
    (`self.ApplyFishes`))
  (return _returnvalue_2))

(fn `UserConstructionScript`
  (`self.ApplyFishes`))
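; BP_Day is a looping day clock that tracks progress through a cycle of set Duration.
; Tick feeds delta seconds into AddProgress, which advances Progress and wraps it by modulo at Duration.
; GetAlpha returns Progress as a fraction of Duration, and GetPeriod scales that fraction by the enum entry count to select one of four day periods.
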(event `self.ReceiveTick`
  (params (DeltaSeconds :type "Float (single-precision)"))
  (`self.AddProgress` DeltaSeconds))

(fn `AddProgress`
  (params (Progress :type "Float (double-precision)"))
  (set `self.Progress` (mod (+ (`KismetMathLibrary.FMax` Progress) (`self.Progress`)) (`self.Duration`))))

(fn `GetAlpha`
  (returns (Alpha :type "Float (double-precision)"))
  (return (/ (`self.Progress`) (`self.Duration`))))

(fn `GetPeriod`
  (returns (Period :type "/Game/Database/EN_Period Enum"))
  (return (select `int` (`KismetMathLibrary.FTrunc` (* (`self.GetAlpha`) (enumcount `/Game/Database/EN_Period`))) :`0` "NewEnumerator4" :`1` "NewEnumerator5" :`2` "NewEnumerator6" :`3` "NewEnumerator7" :!type "/Game/Database/EN_Period Enum")))

(fn `UserConstructionScript`)
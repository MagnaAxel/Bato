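; BP_Cargo is a cargo object that displays its stored quantity through up to four cargo components.
; ApplyQuantity shows each component whose index is below Quantity and hides the rest, running at construction and after every change.
; AddQuantity and ResetQuantity route through SetQuantity, which stores the value and refreshes the visuals.
; Only AddQuantity clamps the value to the four-slot range.
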(fn `AddQuantity`
  (params (Quantity :type Integer))
  (returns (Success :type Boolean))
  (bind _success (`self.SetQuantity` (`KismetMathLibrary.Clamp` (+ (`self.Quantity`) Quantity) 0 4)))
  (return _success))

(fn `ApplyQuantity`
  (for (_array_element _array_index) (`|MakeArray` (`self.Cargo1`) (`self.Cargo2`) (`self.Cargo3`) (`self.Cargo4`))
    (`SceneComponent.SetVisibility` _array_element (< _array_index (`self.Quantity`)) false)))

(fn `GetQuantity`
  (returns (Success :type Boolean) (Quantity :type Integer))
  (return true (`self.Quantity`)))

(fn `ResetQuantity`
  (returns (Success :type Boolean))
  (bind _success (`self.SetQuantity` 0))
  (return _success))

(fn `SetQuantity`
  (params (Quantity :type Integer))
  (returns (Success :type Boolean))
  (set `self.Quantity` Quantity)
  (`self.ApplyQuantity`)
  (return true))

(fn `UserConstructionScript`
  (`self.ApplyQuantity`))
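; BP_FishingRod is a fishing rod actor that drops a hook and credits its owner with catches.
; Fish starts a timeline, guarded by a Fishing flag, that drives the hook's swept vertical offset and the spline mesh line's end, scaled by Depness.
; On overlap, it sends CatchMessage to the other actor and, if accepted, adds one to the owner's quantity.
; Tick keeps the line's world rotation zeroed.
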(event `self.ReceiveTick`
  (params (DeltaSeconds :type "Float (single-precision)"))
  (`SceneComponent.K2_SetWorldRotation` :`self` (`self.SplineMesh`)))

(event `self.ReceiveActorBeginOverlap`
  (params (OtherActor :type "Actor Object Reference"))
  (bind _success (message `/Game/Blueprints/Gameplay/IN_Catchable.Catch` OtherActor))
  (if _success
    (message `/Game/Blueprints/Gameplay/IN_Cargo.AddQuantity` (`self.GetOwner`) 1)))

(fn `Fish`
  (returns (Success :type Boolean))
  (if (not (`self.Fishing`))
    (set `self.Fishing` true)
    (`TimelineComponent.PlayFromStart` (`self.TimelineFishing`))
    (return true)))

(fn `UserConstructionScript`)
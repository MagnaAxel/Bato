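; BP_Bato is a controllable pawn, apparently a boat, that moves, fishes, stores fish and fires a cannon.
; Move applies forward movement input and interpolates rotation at a rate set by Maneuverability, while Look adds controller yaw.
; Cast, Pull, Shoot, AddFish and RemoveFish forward messages to the FishingRod, Cannon and Cargo child actors and return their results, keeping that logic outside the pawn.
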(fn `AddFish`
  (params (Fish :type "/Game/Database/Fish/EN_Fish Enum" :default "NewEnumerator0"))
  (returns (Success :type Boolean))
  (bind _success (message `/Game/Blueprints/Gameplay/Cargo/IN_Cargo.AddFish` (`ChildActorComponent.ChildActor` (`self.Cargo`)) Fish))
  (return _success))

(fn `Cast`
  (returns (Success :type Boolean))
  (bind _success (message `/Game/Blueprints/Gameplay/FishingRod/IN_FishingRod.Cast` (`ChildActorComponent.ChildActor` (`self.FishingRod`))))
  (return _success))

(fn `Look`
  (params (Yaw :type "Float (double-precision)"))
  (returns (Success :type Boolean))
  (`self.AddControllerYawInput` Yaw)
  (return true))

(fn `Move`
  (params (Vector2D :type "Vector2D Structure"))
  (returns (Success :type Boolean))
  (bind (_x _y) (`KismetMathLibrary.BreakVector2D` Vector2D))
  (bind _returnvalue (`self.K2_GetActorRotation`))
  (`|ExecutionSequence`
    (:`then_0`
      (`self.AddMovementInput` (* (`self.GetActorForwardVector`) _x)))
    (:`then_1`
      (`self.K2_SetActorRotation` (`KismetMathLibrary.RInterpTo` _returnvalue (`KismetMathLibrary.ComposeRotators` _returnvalue (* (struct :`Yaw` 90.0) _y)) (`GameplayStatics.GetWorldDeltaSeconds`) (`self.Maneuverability`)))
      (return true))))

(fn `Pull`
  (params (Direction :type "/Game/Database/EN_Pull Enum" :default "NewEnumerator0"))
  (returns (Success :type Boolean))
  (bind _success (message `/Game/Blueprints/Gameplay/FishingRod/IN_FishingRod.Pull` (`ChildActorComponent.ChildActor` (`self.FishingRod`)) Direction))
  (return _success))

(fn `RemoveFish`
  (params (Fish :type "/Game/Database/Fish/EN_Fish Enum" :default "NewEnumerator0"))
  (returns (Success :type Boolean))
  (bind _success (message `/Game/Blueprints/Gameplay/Cargo/IN_Cargo.RemoveFish` (`ChildActorComponent.ChildActor` (`self.Cargo`)) Fish))
  (return _success))

(fn `Shoot`
  (returns (Success :type Boolean))
  (bind _success (message `/Game/Blueprints/Gameplay/Cannon/IN_Cannon.Shoot` (`ChildActorComponent.ChildActor` (`self.Cannon`))))
  (return _success))

(fn `UserConstructionScript`)
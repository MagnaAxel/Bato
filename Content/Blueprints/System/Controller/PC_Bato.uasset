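; Player controller that turns Enhanced Input actions for moving, looking, fishing, pulling and shooting into commands for the controlled pawn.
; Each action is forwarded as a message call, so the pawn decides how to respond.
; Pull input is truncated to whole-number axes and looked up in a map of four cardinal vectors to send a direction enum instead of a raw vector.
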(event `EnhancedInput|/Game/Blueprints/System/Controller/IA_Move`
  (params (ActionValue :type "Vector2D Structure") (ElapsedSeconds :type "Float (double-precision)") (TriggeredSeconds :type "Float (double-precision)") (InputAction :type "InputAction Object Reference" :default "/Game/Blueprints/System/Controller/IA_Move.IA_Move"))
  (:`Triggered`
    (message `/Game/Blueprints/Gameplay/Bato/IN_Bato.Move` (`self.K2_GetPawn`) ActionValue)))

(event `EnhancedInput|/Game/Blueprints/System/Controller/IA_Look`
  (params (ActionValue :type "Float (double-precision)") (ElapsedSeconds :type "Float (double-precision)") (TriggeredSeconds :type "Float (double-precision)") (InputAction :type "InputAction Object Reference" :default "/Game/Blueprints/System/Controller/IA_Look.IA_Look"))
  (:`Triggered`
    (message `/Game/Blueprints/Gameplay/Bato/IN_Bato.Look` (`self.K2_GetPawn`) ActionValue)))

(event `EnhancedInput|/Game/Blueprints/System/Controller/IA_Fish`
  (params (ActionValue :type Boolean) (ElapsedSeconds :type "Float (double-precision)") (TriggeredSeconds :type "Float (double-precision)") (InputAction :type "InputAction Object Reference" :default "/Game/Blueprints/System/Controller/IA_Fish.IA_Fish"))
  (:`Triggered`
    (message `/Game/Blueprints/Gameplay/FishingRod/IN_FishingRod.Cast` (`self.K2_GetPawn`))))

(event `EnhancedInput|/Game/Blueprints/System/Controller/IA_Pull`
  (params (ActionValue :type "Vector2D Structure") (ElapsedSeconds :type "Float (double-precision)") (TriggeredSeconds :type "Float (double-precision)") (InputAction :type "InputAction Object Reference" :default "/Game/Blueprints/System/Controller/IA_Pull.IA_Pull"))
  (bind (_x _y) (`KismetMathLibrary.BreakVector2D` ActionValue))
  (:`Triggered`
    (message `/Game/Blueprints/Gameplay/FishingRod/IN_FishingRod.Pull` (`self.K2_GetPawn`) (`BlueprintMapLibrary.Map_Find` (`|MakeMap` (1.0 0.0) "NewEnumerator0" (0.0 1.0) "NewEnumerator1" (-1.0 0.0) "NewEnumerator2" (0.0 -1.0) "NewEnumerator3" :!type "Vector2D Structure" :!valuetype "/Game/Database/EN_Direction Enum") (`KismetMathLibrary.MakeVector2D` (`KismetMathLibrary.Conv_IntToDouble` (`KismetMathLibrary.FTrunc` _x)) (`KismetMathLibrary.Conv_IntToDouble` (`KismetMathLibrary.FTrunc` _y)))))))

(event `EnhancedInput|/Game/Blueprints/System/Controller/IA_Shoot`
  (params (ActionValue :type Boolean) (ElapsedSeconds :type "Float (double-precision)") (TriggeredSeconds :type "Float (double-precision)") (InputAction :type "InputAction Object Reference" :default "/Game/Blueprints/System/Controller/IA_Shoot.IA_Shoot"))
  (:`Triggered`
    (message `/Game/Blueprints/Gameplay/Cannon/IN_Cannon.Shoot` (`self.K2_GetPawn`))))

(fn `UserConstructionScript`)
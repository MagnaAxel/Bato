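; Game instance that manages local players based on connected input devices.
; On Init it retries each tick until the game mode is valid, then binds to device connection changes and creates a player for each active platform user.
; A new connection creates another player.
; Any other state change removes players whose platform user has no input devices left, destroying their pawns.
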(event `self.ReceiveInit`
  (`/Engine/EditorBlueprintResources/StandardMacros.IsValid` (`GameplayStatics.GetGameMode`) :!label _label
    (:`Is Valid`
      (add `self.OnInputDeviceConnectionChange` (delegate `Event_OnInputDeviceConnectionChange`))
      (bind _outusers (`InputDeviceLibrary.GetAllActiveUsers`))
      (for _array_element _outusers
        (`GameplayStatics.CreatePlayerFromPlatformUser` _array_element)))
    (:`Is Not Valid`
      (`KismetSystemLibrary.DelayUntilNextTick`)
      (goto _label))))

(event `Event_OnInputDeviceConnectionChange`
  (params (NewConnectionState :type "EInputDeviceConnectionState Enum" :default "Invalid") (PlatformUserId :type "PlatformUserId Structure") (InputDeviceId :type "InputDeviceId Structure"))
  (switch `EInputDeviceConnectionState` NewConnectionState
    (:`Invalid`
      (bind _outactors (`GameplayStatics.GetAllActorsOfClass` "/Script/Engine.PlayerController" :!label _label_2))
      (for _array_element _outactors
        (bind _outinputdevices (`InputDeviceLibrary.GetAllInputDevicesForUser` (`PlayerController.GetPlatformUserId` _array_element)))
        (if (`KismetArrayLibrary.Array_IsEmpty` _outinputdevices)
          (`GameplayStatics.RemovePlayer` _array_element true))))
    (:`Unknown`
      (goto _label_2))
    (:`Disconnected`
      (goto _label_2))
    (:`Connected`
      (`GameplayStatics.CreatePlayer` -1))))
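; Function library that computes the height and surface normal of summed, time-animated Gerstner-style waves at a given coordinate.
; GetGerstner derives a phase from each wave's direction, length, speed, offset and game time, returning height and a 2D slope.
; Height is a sine sharpened by a steepness exponent without horizontal displacement, while the slope uses a simpler cosine term.
; GetWave sums both over a wave array and builds the normal from the negated slope.
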(fn `GetGerstner`
  (params (WorldPosition :type "Vector2D Structure") (Wave :type "/Game/Blueprints/System/ST_Wave Structure (by ref)"))
  (returns (Height :type "Float (double-precision)") (Derivative :type "Vector2D Structure"))
  (locals (Coordinate :type "Vector2D Structure") (Direction :type "Vector2D Structure") (Amplitude :type "Float (double-precision)") (Length :type "Float (double-precision)") (Speed :type "Float (double-precision)") (Offset :type "Float (double-precision)") (Steepness :type "Float (double-precision)"))
  (bind (_direction _amplitude _length _speed _offset _steepness) (break `/Game/Blueprints/System/ST_Wave` Wave))
  (bind _direction_2 (`local.Direction`))
  (bind _amplitude_2 (`local.Amplitude`))
  (bind _steepness_2 (`local.Steepness`))
  (bind _returnvalue (/ (`KismetMathLibrary.MultiplyByPi` 2.0) (`local.Length`)))
  (bind _returnvalue_2 (+ (- (* (`KismetMathLibrary.DotProduct2D` _direction_2 (`local.Coordinate`)) _returnvalue) (* (* _returnvalue (`local.Speed`)) (`GameplayStatics.GetTimeSeconds` null))) (`local.Offset`)))
  (`|ExecutionSequence`
    (:`then_0`
      (set `local.Coordinate` WorldPosition))
    (:`then_1`
      (set `local.Direction` _direction))
    (:`then_2`
      (set `local.Amplitude` _amplitude))
    (:`then_3`
      (set `local.Length` _length))
    (:`then_4`
      (set `local.Speed` _speed))
    (:`then_5`
      (set `local.Offset` _offset))
    (:`then_6`
      (set `local.Steepness` _steepness))
    (:`then_7`
      (return (* (`KismetMathLibrary.MultiplyMultiply_FloatFloat` (/ (+ (`KismetMathLibrary.Sin` (* (`KismetMathLibrary.MultiplyByPi` 2.0) _returnvalue_2)) 1.0) 2.0) (+ _steepness_2 1.0)) _amplitude_2) (`KismetMathLibrary.MakeVector2D` (* (* (* (* _amplitude_2 _returnvalue) (+ _steepness_2 1.0)) (`KismetMathLibrary.Cos` (* (`KismetMathLibrary.MultiplyByPi` 2.0) _returnvalue_2))) (`KismetMathLibrary.BreakVector2D` _direction_2)) (* (* (* (* _amplitude_2 _returnvalue) (+ _steepness_2 1.0)) (`KismetMathLibrary.Cos` (* (`KismetMathLibrary.MultiplyByPi` 2.0) _returnvalue_2))) (`.Y` (`KismetMathLibrary.BreakVector2D` _direction_2))))))))

(fn `GetWave`
  (params (Coordinate :type "Vector2D Structure (by ref)") (Waves :type "Array of /Game/Blueprints/System/ST_Wave Structure"))
  (returns (Height :type "Float (double-precision)") (Normal :type "Vector Structure"))
  (locals (LocalHeight :type "Float (double-precision)" :default 0.0) (LocalDerivative :type "Vector2D Structure"))
  (for _array_element Waves
    (bind (_height _derivative) (`self.GetGerstner` Coordinate _array_element))
    (set `local.LocalHeight` (+ (`local.LocalHeight`) _height))
    (set `local.LocalDerivative` (+ (`local.LocalDerivative`) _derivative)))
  (return (`local.LocalHeight`) (`KismetMathLibrary.Normal` (`KismetMathLibrary.Conv_Vector2DToVector` (`KismetMathLibrary.Negated2D` (`local.LocalDerivative`)) 1.0))))
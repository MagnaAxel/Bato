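; Wave function library that computes water height and surface normal at a 2D coordinate from arrays of waves, islands and storms.
; GetWave sums time-animated GetGerstner waves, which are steepness-sharpened sines with vertical displacement only, and builds the normal from their summed derivatives.
; Radial falloffs scale height only: the minimum across islands times the maximum across storms, both via GetAttenuation, leaving GetAmplification unused.
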(fn `GetAmplification`
  (params (Coordinate :type "Vector2D Structure") (Modifier :type "/Game/Database/ST_Modifier Structure"))
  (returns (Attenuation :type "Float (double-precision)"))
  (bind (_location _innerradius _outerradius _attenuation) (break `/Game/Database/ST_Modifier` Modifier))
  (return (`KismetMathLibrary.Lerp` 1.0 _attenuation (`KismetMathLibrary.FClamp` (/ (- (`KismetMathLibrary.Distance2D` Coordinate _location) _outerradius) (- _innerradius _outerradius))))))

(fn `GetAttenuation`
  (params (Coordinate :type "Vector2D Structure") (Island :type "/Game/Database/ST_Modifier Structure"))
  (returns (Attenuation :type "Float (double-precision)"))
  (bind (_location _innerradius _outerradius _attenuation) (break `/Game/Database/ST_Modifier` Island))
  (return (`KismetMathLibrary.Lerp` 1.0 _attenuation (`KismetMathLibrary.FClamp` (/ (- (`KismetMathLibrary.Distance2D` Coordinate _location) _outerradius) (- _innerradius _outerradius))))))

(fn `GetGerstner`
  (params (Coordinate :type "Vector2D Structure") (Wave :type "/Game/Database/ST_Wave Structure (by ref)"))
  (returns (Height :type "Float (double-precision)") (Derivative :type "Vector2D Structure"))
  (locals (Coordinate_ :type "Vector2D Structure") (Direction :type "Float (double-precision)") (Amplitude :type "Float (double-precision)") (Length :type "Float (double-precision)") (Speed :type "Float (double-precision)") (Offset :type "Float (double-precision)") (Steepness :type "Float (double-precision)"))
  (bind (_direction _amplitude _length _speed _offset _steepness) (break `/Game/Database/ST_Wave` Wave))
  (bind _amplitude_2 (`local.Amplitude`))
  (bind _steepness_2 (`local.Steepness`))
  (bind _returnvalue (/ (`KismetMathLibrary.MultiplyByPi` 2.0) (`local.Length`)))
  (bind _returnvalue_2 (* (`local.Direction`) (`KismetMathLibrary.MultiplyByPi` 2.0)))
  (bind _returnvalue_3 (`KismetMathLibrary.MakeVector2D` (`KismetMathLibrary.Cos` _returnvalue_2) (`KismetMathLibrary.Sin` _returnvalue_2)))
  (bind _returnvalue_4 (+ (- (* (`KismetMathLibrary.DotProduct2D` _returnvalue_3 (`local.Coordinate_`)) _returnvalue) (* (* _returnvalue (`local.Speed`)) (`GameplayStatics.GetTimeSeconds` null))) (`local.Offset`)))
  (`|ExecutionSequence`
    (:`then_0`
      (set `local.Coordinate_` Coordinate))
    (:`then_1`
      (set `local.Direction` _direction))
    (:`then_2`
      (set `local.Amplitude` _amplitude))
    (:`then_3`
      (set `local.Length` _length))
    (:`then_4`
      (set `local.Speed` _speed))
    (:`then_5`
      (set `local.Offset` _offset))
    (:`then_6`
      (set `local.Steepness` _steepness))
    (:`then_7`
      (return (* (`KismetMathLibrary.MultiplyMultiply_FloatFloat` (/ (+ (`KismetMathLibrary.Sin` (* (`KismetMathLibrary.MultiplyByPi` 2.0) _returnvalue_4)) 1.0) 2.0) (+ _steepness_2 1.0)) _amplitude_2) (`KismetMathLibrary.MakeVector2D` (* (* (* (* _amplitude_2 _returnvalue) (+ _steepness_2 1.0)) (`KismetMathLibrary.Cos` (* (`KismetMathLibrary.MultiplyByPi` 2.0) _returnvalue_4))) (`KismetMathLibrary.BreakVector2D` _returnvalue_3)) (* (* (* (* _amplitude_2 _returnvalue) (+ _steepness_2 1.0)) (`KismetMathLibrary.Cos` (* (`KismetMathLibrary.MultiplyByPi` 2.0) _returnvalue_4))) (`.Y` (`KismetMathLibrary.BreakVector2D` _returnvalue_3))))))))

(fn `GetIsland`
  (params (Coordinate :type "Vector2D Structure") (Islands :type "Array of /Game/Database/ST_Modifier Structure"))
  (returns (Attenuation :type "Float (double-precision)"))
  (locals (LocalAttenuation :type "Float (double-precision)" :default 1.0))
  (for _array_element Islands
    (set `local.LocalAttenuation` (`KismetMathLibrary.FMin` (`self.GetAttenuation` Coordinate _array_element) (`local.LocalAttenuation`))))
  (return (`local.LocalAttenuation`)))

(fn `GetStorm`
  (params (Coordinate :type "Vector2D Structure") (Storms :type "Array of /Game/Database/ST_Modifier Structure"))
  (returns (Amplification :type "Float (double-precision)"))
  (locals (LocalAmplification :type "Float (double-precision)" :default 1.0))
  (for _array_element Storms
    (set `local.LocalAmplification` (`KismetMathLibrary.FMax` (`self.GetAttenuation` Coordinate _array_element) (`local.LocalAmplification`))))
  (return (`local.LocalAmplification`)))

(fn `GetWave`
  (params (Coordinate :type "Vector2D Structure (by ref)") (Waves :type "Array of /Game/Database/ST_Wave Structure") (Islands :type "Array of /Game/Database/ST_Modifier Structure") (Storms :type "Array of /Game/Database/ST_Modifier Structure"))
  (returns (Height :type "Float (double-precision)") (Normal :type "Vector Structure"))
  (locals (LocalHeight :type "Float (double-precision)" :default 0.0) (LocalDerivative :type "Vector2D Structure"))
  (for _array_element Waves
    (bind (_height _derivative) (`self.GetGerstner` Coordinate _array_element))
    (set `local.LocalHeight` (+ (`local.LocalHeight`) _height))
    (set `local.LocalDerivative` (+ (`local.LocalDerivative`) _derivative)))
  (return (* (`local.LocalHeight`) (`self.GetIsland` Coordinate Islands) (`self.GetStorm` Coordinate Storms)) (`KismetMathLibrary.Normal` (`KismetMathLibrary.Conv_Vector2DToVector` (`KismetMathLibrary.Negated2D` (`local.LocalDerivative`)) 1.0))))
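; GSB_Bato holds the shared Waves array that defines the water surface, keeping material visuals and height queries on the same data.
; On construction, ApplyWaveMaterial writes each wave's direction, amplitude, length, speed, offset and steepness into index-suffixed scalar material parameters on StaticMeshActors tagged "Wave".
; GetWave passes a coordinate and that same array to a wave function, returning surface height and normal.
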(fn `ApplyWaveMaterial`
  (bind _outactors (`GameplayStatics.GetAllActorsOfClassWithTag` "/Script/Engine.StaticMeshActor" "Wave"))
  (for _array_element _outactors
    (for (_array_element_2 _array_index) (`self.Waves`)
      (`|ExecutionSequence`
        (:`then_0`
          (bind _staticmeshcomponent (`StaticMeshActor.StaticMeshComponent` _array_element))
          (bind _returnvalue (`KismetStringLibrary.Conv_IntToString` _array_index))
          (bind (_direction _amplitude _length _speed _offset _steepness) (break `/Game/Blueprints/ST_Wave` _array_element_2))
          (bind (_x _y) (`KismetMathLibrary.BreakVector2D` _direction))
          (`MeshComponent.SetScalarParameterValueOnMaterials` _staticmeshcomponent (`KismetStringLibrary.Conv_StringToName` (`KismetStringLibrary.Concat_StrStr` "DirectionX" _returnvalue)) _x))
        (:`then_1`
          (`MeshComponent.SetScalarParameterValueOnMaterials` _staticmeshcomponent (`KismetStringLibrary.Conv_StringToName` (`KismetStringLibrary.Concat_StrStr` "DirectionY" _returnvalue)) _y))
        (:`then_2`
          (`MeshComponent.SetScalarParameterValueOnMaterials` _staticmeshcomponent (`KismetStringLibrary.Conv_StringToName` (`KismetStringLibrary.Concat_StrStr` "Amplitude" _returnvalue)) _amplitude))
        (:`then_3`
          (`MeshComponent.SetScalarParameterValueOnMaterials` _staticmeshcomponent (`KismetStringLibrary.Conv_StringToName` (`KismetStringLibrary.Concat_StrStr` "Length" _returnvalue)) _length))
        (:`then_4`
          (`MeshComponent.SetScalarParameterValueOnMaterials` _staticmeshcomponent (`KismetStringLibrary.Conv_StringToName` (`KismetStringLibrary.Concat_StrStr` "Speed" _returnvalue)) _speed))
        (:`then_5`
          (`MeshComponent.SetScalarParameterValueOnMaterials` _staticmeshcomponent (`KismetStringLibrary.Conv_StringToName` (`KismetStringLibrary.Concat_StrStr` "Offset" _returnvalue)) _offset))
        (:`then_6`
          (`MeshComponent.SetScalarParameterValueOnMaterials` _staticmeshcomponent (`KismetStringLibrary.Conv_StringToName` (`KismetStringLibrary.Concat_StrStr` "Steepness" _returnvalue)) _steepness))))))

(fn `GetWave`
  (params (Coordinate :type "Vector2D Structure"))
  (returns (Height :type "Float (double-precision)") (Normal :type "Vector Structure"))
  (bind (_height _normal) (`/Game/Blueprints/FL_Gerstner.GetWave` Coordinate (`self.Waves`)))
  (return _height _normal))

(fn `UserConstructionScript`
  (`self.ApplyWaveMaterial`))
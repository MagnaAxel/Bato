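; SubPawn is an actor that follows the possession of its parent Pawn, apparently as a Child Actor attached to it.
; Its construction script binds to the parent Pawn's controller-changed delegate.
; On a change it fires empty Unpossessed and Possessed hook events for valid old and new controllers.
; It clears PlayerState after Unpossessed, caches the new controller's before Possessed, and exposes it through GetPlayerState.
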(event `Possessed`
  (params (NewController :type "Controller Object Reference (by ref)")))

(event `Unpossessed`
  (params (OldController :type "Controller Object Reference (by ref)")))

(fn `GetPlayerState`
  (returns (PlayerState :type "PlayerState Object Reference"))
  (return (`self.PlayerState`)))

(fn `OnReceiveControllerChangedDelegate`
  (params (Pawn :type "Pawn Object Reference") (OldController :type "Controller Object Reference") (NewController :type "Controller Object Reference"))
  (`|ExecutionSequence`
    (:`then_0`
      (`/Engine/EditorBlueprintResources/StandardMacros.IsValid` OldController
        (:`Is Valid`
          (`self.Unpossessed` OldController)
          (set `self.PlayerState` null))))
    (:`then_1`
      (`/Engine/EditorBlueprintResources/StandardMacros.IsValid` NewController
        (:`Is Valid`
          (set `self.PlayerState` (`Controller.PlayerState` NewController))
          (`self.Possessed` NewController))))))

(fn `UserConstructionScript`
  (bind _aspawn (cast `Pawn` (`self.GetParentActor`)))
  (add `Pawn.ReceiveControllerChangedDelegate` _aspawn (`|CreateDelegate` :!event `OnReceiveControllerChangedDelegate`)))